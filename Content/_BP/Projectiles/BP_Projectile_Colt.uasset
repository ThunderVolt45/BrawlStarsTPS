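; Colt projectile that applies a gameplay effect to actors it overlaps.
; On sphere overlap it ignores its instigator and itself, then applies its stored SpecHandle to the other actor's Ability System Component, if one exists.
; It destroys itself only after a short fixed lifetime, so a hit does not stop it from affecting further actors.
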(event OnComponentBeginOverlap(Sphere)
  (params (OverlappedComponent :type Primitive%20Component%20Object%20Reference) (OtherActor :type Actor%20Object%20Reference) (OtherComp :type Primitive%20Component%20Object%20Reference) (OtherBodyIndex :type Integer) (bFromSweep :type Boolean) (SweepResult :type Hit%20Result%20Structure%20%28by%20ref%29))
  (bind _returnvalue (Actor|GetComponentbyClass OtherActor "/Script/GameplayAbilities.AbilitySystemComponent"))
  (if (and (!= OtherActor (Game|GetInstigator)) (!= OtherActor self))
    (Utilities|IsValid _returnvalue
      (:Is%20Valid
        (GameplayEffects|ApplyGameplayEffectSpecToSelf _returnvalue (Variables|Default|GetSpecHandle))))))

(event EventBeginPlay
  (Utilities|FlowControl|Delay 3.0)
  (Actor|DestroyActor))

(fn ConstructionScript)