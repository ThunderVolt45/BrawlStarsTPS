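; Colt's attack gameplay ability, which fires projectiles from his left and right muzzles.
; On activation it applies cooldown, ammo cost and damage effects, then plays a montage whose gameplay events trigger each muzzle's shot.
; CreateProjectile spawns BP_Projectile_Colt at the chosen muzzle, handing it a GE_Damage spec with a set-by-caller magnitude.
; The ability ends when the montage completes or is interrupted.
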(event Ability|EventActivateAbility
  (Class|BrawlGameplayAbility|ApplyEffecttoSelf "/Game/_BP/Abilities/Effects/GE_Cooldown.GE_Cooldown_C" "(TagName=\"Data.Cooldown\")" (Variables|Default|GetCooldown))
  (Class|BrawlGameplayAbility|ApplyEffecttoSelf :EffectClass "/Game/_BP/Abilities/Effects/GE_AmmoCost.GE_AmmoCost_C" :Magnitude (Variables|Default|GetAmmoCost))
  (Class|BrawlGameplayAbility|ApplyDamageEffect 0 "/Game/_BP/Abilities/Effects/GE_Damage.GE_Damage_C" (Variables|Default|GetDamage%20Amount))
  (|PlayMontageandWaitProxy "None" (Variables|Default|GetMontage%20to%20Play) 1.0 "None" true 1.0 0.0 false
    (:then
      (Ability|Tasks|WaitGameplayEvent (Variables|Default|GetEvent%20to%20Wait%20Right) 0
        (:then
          (Ability|Tasks|WaitGameplayEvent (Variables|Default|GetEvent%20to%20Wait%20Left) 0
            (:EventReceived
              (CallFunction|CreateProjectile true))))
        (:EventReceived
          (CallFunction|CreateProjectile false))))
    (:OnCompleted
      (Ability|EndAbility :!label _label))
    (:OnInterrupted
      (goto _label))))

(event Ability|EventOnEndAbility
  (params (bWasCancelled :type Boolean)))

(fn CreateProjectile
  (params (IsLeft :type Boolean))
  (bind _returnvalue (Class|AbilitySystemBlueprintLibrary|AssignSetbyCallerMagnitude (GameplayEffects|MakeOutgoingSpec :self (Ability|GetAbilitySystemComponentfromActorInfo) :GameplayEffectClass "/Game/_BP/Abilities/Effects/GE_Damage.GE_Damage_C") "None" (Variables|Default|GetDamage%20Amount)))
  (bind _asbp_colt (Utilities|Casting|CastToBP_Colt (Ability|GetAvatarActorfromActorInfo)))
  (if IsLeft
    (bind _muzzle (Default|GetLeftMuzzle _asbp_colt))
    (Game|SpawnActorfromClass "/Game/_BP/Projectiles/BP_Projectile_Colt.BP_Projectile_Colt_C" (Math|Transform|MakeTransform (.location _muzzle) (.rotation _muzzle) "1.000000,1.000000,1.000000") "Undefined" "MultiplyWithRoot" 0 _returnvalue 0)
    (else
      (bind _muzzle_2 (Default|GetRightMuzzle _asbp_colt))
      (Game|SpawnActorfromClass "/Game/_BP/Projectiles/BP_Projectile_Colt.BP_Projectile_Colt_C" (Math|Transform|MakeTransform (.location _muzzle_2) (.rotation _muzzle_2) "1.000000,1.000000,1.000000") "Undefined" "MultiplyWithRoot" 0 _returnvalue 0))))